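; BP_Indicador_Luz is an indicator light whose sphere color reflects the state of a referenced trap (Trampa) and the player's proximity.
; The construction script starts the sphere black.
; Every Tick, it turns red if the trap's Cerrado flag is set.
; Otherwise, it measures its own distance to the player character, turning green within a fixed radius and black beyond it.
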(event `self.ReceiveTick`
  (params (DeltaSeconds :type "Float (single-precision)"))
  ; lo primero es que todo el tiempo se verifique si esta cerrada la trampa
  (if (`/Game/Pilar_Marco/BP_Assets/BP_Trampa.cerrado` (`self.Trampa`))
    ; Si està cerrada, el material pasa a rojo
    (`PrimitiveComponent.SetMaterial` (`self.Esfera_Luz`) 0 "/Game/Pilar_Marco/Materials/M_Color_Rojo.M_Color_Rojo")
    (else
      ; si  no, significa que esta abierta, entonces buscamos al character para comparar la distancia de aquel con el gas toxico
      (bind _asbp_third_person_character (cast `/Game/ThirdPerson/Blueprints/BP_ThirdPersonCharacter` (`GameplayStatics.GetPlayerCharacter` 0)))
      ; guardamos esa distancia en una nueva variable
      (set `self.Distancia_Player` (`self.GetDistanceTo` _asbp_third_person_character))
      ; si es menor, significa que estamos cerca, entonces sel material pasa a ser verde
      (if (<= (`self.Distancia_Player`) 400.0)
        (`PrimitiveComponent.SetMaterial` (`self.Esfera_Luz`) 0 "/Game/Pilar_Marco/Materials/M_Color_Verde.M_Color_Verde")
        (else
          ; si es falso, significa que estamos alejados, entonces se pasa el material a negro
          (`PrimitiveComponent.SetMaterial` (`self.Esfera_Luz`) 0 "/Game/Pilar_Marco/Materials/M_Color_Negro.M_Color_Negro"))))))

(fn `UserConstructionScript`
  (`PrimitiveComponent.SetMaterial` (`self.Esfera_Luz`) 0 "/Game/Pilar_Marco/Materials/M_Color_Negro.M_Color_Negro"))