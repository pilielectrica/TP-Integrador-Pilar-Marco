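; BP_Trampa is a two-door trap actor that closes and releases toxic gas.
; Overlapping its middle collision box, or starting play with Cerrado set, fires a shared DoOnce.
; It instantly drops itself and the referenced front door along Z, then flips the Cerrado and Abierto flags.
; After a short delay it spawns BP_Gas_Tpxico at the Location variable, intended to sit between the doors.
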(event `self.ReceiveBeginPlay`
  ; primero que todo decimos verificamos si esta abierto o cerrado
  (if (`self.cerrado`)
    ; lo siguiente va a hacerse una sola vez porque si no habrà bugs
    (`/Engine/EditorBlueprintResources/StandardMacros.DoOnce` false :!label _label
      (:`Completed`
        ; reducimos la posicion de la puerta frontal de la trampa en z para que toque el suelo
        (`self.K2_AddActorLocalOffset` (`self.Ref_Puerta_Frente`) (0.0 0.0 -200.0) false false)
        ; y tambien la posicion z de esta trampa
        (`self.K2_AddActorLocalOffset` (0.0 0.0 -200.0))
        ; pasamos cerrado a verdadero y abierto a falso
        (set `self.cerrado` true)
        (set `self.abierto` false)
        ; despuès de 2 segundos el gas toxico habrà aparecido en una posicion determinada, entre medio de las dos puertas que conforman la trampa
        (`KismetSystemLibrary.Delay` 2.0)
        (`|SpawnActorFromClass` "/Game/bp/BP_Gas_Tpxico.BP_Gas_Tpxico_C" (`KismetMathLibrary.MakeTransform` (`self.Location`)) "Undefined" "MultiplyWithRoot" null null)))))

(event `self.ReceiveActorBeginOverlap`
  (params (OtherActor :type "Actor Object Reference")))

(event `self.ReceiveTick`
  (params (DeltaSeconds :type "Float (single-precision)")))

(event `self.Box_colission.OnComponentBeginOverlap`
  (params (OverlappedComponent :type "PrimitiveComponent Object Reference") (OtherActor :type "Actor Object Reference") (OtherComp :type "PrimitiveComponent Object Reference") (OtherBodyIndex :type Integer) (bFromSweep :type Boolean) (SweepResult :type "HitResult Structure (by ref)"))
  ; a partir de acà la lògica se aplica a cuando se colisiona contra un collider que està puesto justo en el medio de la trampa
  (goto _label))

(fn `UserConstructionScript`)